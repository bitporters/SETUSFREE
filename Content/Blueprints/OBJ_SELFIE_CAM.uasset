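; Selfie camera actor that gives the player a front-facing view of their pawn while the Down key is held.
; Every tick it moves to a point just ahead of the controlled pawn along its forward vector and rotates to look back at it.
; Pressing the key blends the player controller's view target to this actor, and releasing it blends back to the pawn.
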(event `self.ReceiveBeginPlay`)

(event `self.ReceiveActorBeginOverlap`
  (params (OtherActor :type "Actor Object Reference")))

(event `self.ReceiveTick`
  (params (DeltaSeconds :type "Float (single-precision)"))
  (bind _returnvalue (`Controller.K2_GetPawn` (`GameplayStatics.GetPlayerController` 0)))
  (bind _returnvalue_2 (`self.K2_GetActorLocation` _returnvalue))
  (bind _returnvalue_3 (+ _returnvalue_2 (* (`self.GetActorForwardVector` _returnvalue) 100.0)))
  (`SceneComponent.K2_SetWorldLocation` _returnvalue_3)
  (`self.SetActorRotation` (`KismetMathLibrary.FindLookAtRotation` _returnvalue_3 _returnvalue_2)))

(event `Key|Down`
  (bind _returnvalue (`GameplayStatics.GetPlayerController` 0))
  (:`Pressed`
    (`PlayerController.SetViewTargetWithBlend` _returnvalue self 0.1 "VTBlend_Linear" 0.0 false))
  (:`Released`
    (`PlayerController.SetViewTargetWithBlend` _returnvalue (`Controller.K2_GetPawn` _returnvalue) 0.1 "VTBlend_Linear" 0.0 false)))

(fn `UserConstructionScript`)