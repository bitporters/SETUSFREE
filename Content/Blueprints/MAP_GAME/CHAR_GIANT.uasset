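; Giant monster character that hunts and squishes players, either AI-driven or possessed through BP_CONTROLLER_SETUSFREE with move/turn input.
; On authority, the AI patrols random points on a timer, paused by a cooldown after sighting an unhidden player; PawnSensing sends it toward seen players or noises.
; Moving into a player triggers their suicide.
; Remote or possessed instances run a timer for proximity footstep shakes, rumbles and one-shot screams at closing distances.
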(event `self.ReceiveBeginPlay`
  (cast `/Game/Blueprints/MAP_GAME/BP_CONTROLLER_SETUSFREE` (`self.GetController`)
    (:`then`
      (`GameplayStatics.PlaySoundAtLocation` "/Game/RESOURCES/Sounds/sfx_scream.sfx_scream" (`SceneComponent.K2_GetComponentLocation` (`self.mouth`)) 1.0 0.1)
      (`KismetSystemLibrary.K2_SetTimer` null "DO_SHAKES" 0.25 true :!label _label))
    (:`CastFailed`
      (`/Engine/EditorBlueprintResources/ActorMacros.Switch Has Authority`
        (:`Authority`
          (`KismetSystemLibrary.K2_SetTimer` null "DO_PATROL" 5.0 true))
        (:`Remote`
          (goto _label))))))

(event `self.ReceiveTick`
  (params (DeltaSeconds :type "Float (single-precision)"))
  (bind _chasingcooldown (`self.ChasingCoolDown`))
  (bind _camera (`self.Camera`))
  (`|ExecutionSequence`
    (:`then_0`
      (if (> _chasingcooldown 0.0)
        (set `self.ChasingCoolDown` (`KismetMathLibrary.FClamp` (- _chasingcooldown DeltaSeconds) 0.0 5.0))))
    (:`then_1`
      (`SceneComponent.K2_SetWorldRotation` _camera (`KismetMathLibrary.FindLookAtRotation` (`SceneComponent.K2_GetComponentLocation` _camera) (`SceneComponent.K2_GetComponentLocation` (`self.Mesh`))) false))))

(event `DO_PATROL`
  (`self.GoToRandomPatrolPoint`))

(event `self.PawnSensing.OnSeePawn`
  (params (Pawn :type "Pawn Object Reference"))
  (bind _returnvalue (`self.GetController`))
  (bind _aschar_player (cast `/Game/Blueprints/MAP_GAME/CHAR_PLAYER` Pawn))
  (if (not (`/Game/Blueprints/MAP_GAME/CHAR_PLAYER.bIsHiddenByTree` _aschar_player))
    (`|ExecutionSequence`
      (:`then_0`
        (`Controller.StopMovement` _returnvalue)
        (`NavigationSystem.SimpleMoveToLocation` _returnvalue (`self.K2_GetActorLocation` _aschar_player)))
      (:`then_1`
        (`GameplayStatics.PlaySoundAtLocation` "/Game/RESOURCES/Sounds/sfx_scream.sfx_scream" (`SceneComponent.K2_GetComponentLocation` (`self.mouth`)) 1.0))
      (:`then_2`
        (set `self.ChasingCoolDown` 10.0)))))

(event `InputAxis|MOVE_FORWARD`
  (params (AxisValue :type "Float (single-precision)"))
  (`self.AddMovementInput` (`SceneComponent.GetForwardVector`) AxisValue))

(event `InputAxis|MOVE_LEFT`
  (params (AxisValue :type "Float (single-precision)"))
  (`self.AddControllerYawInput` AxisValue))

(event `self.Squish.OnComponentBeginOverlap`
  (params (OtherActor :type "Actor Object Reference") (OtherComp :type "PrimitiveComponent Object Reference") (OtherBodyIndex :type Integer) (bFromSweep :type Boolean) (SweepResult :type "EngineTypes.HitResult Structure (by ref)"))
  (if (> (`KismetMathLibrary.VSize` (`MovementComponent.Velocity` (`self.CharacterMovement`))) 0.0)
    (bind _aschar_player (cast `/Game/Blueprints/MAP_GAME/CHAR_PLAYER` OtherActor))
    (`/Game/Blueprints/MAP_GAME/CHAR_PLAYER.Server_Suicide` _aschar_player)
    (`GameplayStatics.PlaySoundAtLocation` "/Game/RESOURCES/Sounds/sfx_SPLAT.sfx_SPLAT" (`SceneComponent.K2_GetComponentLocation`))))

(event `DO_SHAKES`
  (bind _returnvalue (`GameplayStatics.GetPlayerPawn` 0))
  (bind _returnvalue_2 (`SceneComponent.K2_GetComponentLocation`))
  (bind _returnvalue_3 (`KismetMathLibrary.VSize` (- _returnvalue_2 (`self.K2_GetActorLocation` _returnvalue))))
  (if (> (`KismetMathLibrary.VSize` (`MovementComponent.Velocity` (`self.CharacterMovement`))) 0.0)
    (if (< _returnvalue_3 1000.0)
      (`|ExecutionSequence`
        (:`then_0`
          (bind _aschar_player (cast `/Game/Blueprints/MAP_GAME/CHAR_PLAYER` _returnvalue))
          (bind _returnvalue_4 (`Controller.CastToPlayerController` (`self.GetController` _aschar_player)))
          (`PlayerController.ClientStartCameraShake` _returnvalue_4 "/Game/Blueprints/MAP_GAME/CONFIG/MY_CAMERA_SHAKE.MY_CAMERA_SHAKE_C" 1.0 "CameraLocal" (struct))
          (`GameplayStatics.PlaySoundAtLocation` "/Game/RESOURCES/Sounds/EXPLOSION_Sublte_Muffled_Dark__stereo__Cue.EXPLOSION_Sublte_Muffled_Dark__stereo__Cue" _returnvalue_2))
        (:`then_1`
          ;[1 1 1] CLOSE
          (if (`KismetMathLibrary.NearlyEqual_FloatFloat` _returnvalue_3 500.0 100.0)
            (`/Engine/EditorBlueprintResources/StandardMacros.DoOnce` false
              (:`Completed`
                (`GameplayStatics.PlaySoundAttached` "/Game/RESOURCES/Sounds/sfx_scream.sfx_scream" (`self.mouth`) "None" (0.0 0.0 0.0) "KeepRelativeOffset" false 1.0 1.0)))))
        (:`then_2`
          ;[1 1 1] CLOSE
          (if (`KismetMathLibrary.NearlyEqual_FloatFloat` _returnvalue_3 350.0 100.0)
            (`/Engine/EditorBlueprintResources/StandardMacros.DoOnce` false
              (:`Completed`
                (`GameplayStatics.PlaySoundAttached` "/Game/RESOURCES/Sounds/sfx_scream.sfx_scream" (`self.mouth`) "None" (0.0 0.0 0.0) "KeepRelativeOffset" false 1.0 0.5)))))
        (:`then_3`
          ;[1 1 1] CLOSE
          (if (`KismetMathLibrary.NearlyEqual_FloatFloat` _returnvalue_3 100.0 50.0)
            (`/Engine/EditorBlueprintResources/StandardMacros.DoOnce` false
              (:`Completed`
                (`GameplayStatics.PlaySoundAttached` "/Game/RESOURCES/Sounds/sfx_scream.sfx_scream" (`self.mouth`) "None" (0.0 0.0 0.0) "KeepRelativeOffset" false 1.0 0.2)))))))))

(event `self.PawnSensing.OnHearNoise`
  (params (Instigator :type "Pawn Object Reference") (Location :type "Object.Vector Structure (by ref)") (Volume :type "Float (single-precision)"))
  (`GameplayStatics.PlaySoundAtLocation` "/Game/RESOURCES/Sounds/sfx_scream.sfx_scream" (`self.K2_GetActorLocation`))
  (`NavigationSystem.SimpleMoveToLocation` (`self.GetController`) Location))

(fn `GoToRandomPatrolPoint`
  (bind _patrol_points (`self.PATROL_POINTS`))
  (bind _returnvalue (`KismetArrayLibrary.Array_Length` _patrol_points))
  (if (== (`self.ChasingCoolDown`) 0.0)
    (if (> _returnvalue 0)
      (`NavigationSystem.SimpleMoveToLocation` (`self.GetController`) (`self.K2_GetActorLocation` (`KismetArrayLibrary.Array_Get` _patrol_points (`KismetMathLibrary.RandomIntegerInRange` 0 (- _returnvalue 1))))))))

(fn `UserConstructionScript`)