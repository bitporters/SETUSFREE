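; Jetpack pickup actor that spins slowly and grants the player a jetpack.
; Overlapping its sphere sets the jetpack flag on CHAR_PLAYER, before any authority check.
; Only on remote (non-authority) instances, it unhides the player's jetpack object and hides the whole pickup briefly before showing it again.
; A jump sound node is present but unconnected, so no sound plays.
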(event `self.ReceiveBeginPlay`)

(event `self.ReceiveActorBeginOverlap`
  (params (OtherActor :type "Actor Object Reference")))

(event `self.ReceiveTick`
  (params (DeltaSeconds :type "Float (single-precision)"))
  (`SceneComponent.K2_AddLocalRotation` (`self.Cube`) (`KismetMathLibrary.MakeRot` 0.0 (* DeltaSeconds 20.0)) false))

(event `self.Sphere.OnComponentBeginOverlap`
  (params (OtherActor :type "Actor Object Reference") (OtherComp :type "PrimitiveComponent Object Reference") (OtherBodyIndex :type Integer) (bFromSweep :type Boolean) (SweepResult :type "EngineTypes.HitResult Structure (by ref)"))
  (bind _aschar_player (cast `/Game/Blueprints/MAP_GAME/CHAR_PLAYER` OtherActor))
  (set `/Game/Blueprints/MAP_GAME/CHAR_PLAYER.bHasJetPAck` true _aschar_player)
  (`/Engine/EditorBlueprintResources/ActorMacros.Switch Has Authority`
    (:`Remote`
      (`|ExecutionSequence`
        (:`then_0`
          (`SceneComponent.SetHiddenInGame` (`/Game/Blueprints/MAP_GAME/CHAR_PLAYER.objJetPack` _aschar_player) false false))
        (:`then_1`
          (`self.SetActorHiddenInGame` true)
          (`KismetSystemLibrary.Delay` 2.0)
          (`self.SetActorHiddenInGame` false))))))

(fn `UserConstructionScript`)