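; Mushroom pickup that grants the player the ability to explode walls.
; Sphere overlap with a CHAR_PLAYER sets its CanExplodeWall flag.
; Only on the Remote branch of an authority switch, it activates the player's wallbreaker effect, plays a sound and hides the mushroom briefly before showing it again.
; Collision is never disabled, so the hide is purely visual.
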(event `self.ReceiveBeginPlay`)

(event `self.ReceiveActorBeginOverlap`
  (params (OtherActor :type "Actor Object Reference")))

(event `self.ReceiveTick`
  (params (DeltaSeconds :type "Float (single-precision)")))

(event `self.Sphere.OnComponentBeginOverlap`
  (params (OtherActor :type "Actor Object Reference") (OtherComp :type "PrimitiveComponent Object Reference") (OtherBodyIndex :type Integer) (bFromSweep :type Boolean) (SweepResult :type "EngineTypes.HitResult Structure (by ref)"))
  (bind _aschar_player (cast `/Game/Blueprints/MAP_GAME/CHAR_PLAYER` OtherActor))
  (set `/Game/Blueprints/MAP_GAME/CHAR_PLAYER.bCanExplodeWall` true _aschar_player)
  (`/Engine/EditorBlueprintResources/ActorMacros.Switch Has Authority`
    (:`Remote`
      (`|ExecutionSequence`
        (:`then_0`
          (`ActorComponent.Activate` (`/Game/Blueprints/MAP_GAME/CHAR_PLAYER.p_wallbreaker` _aschar_player) false)
          (`GameplayStatics.PlaySoundAtLocation` "/Game/RESOURCES/Sounds/Jump_Enemy_Cue.Jump_Enemy_Cue" (`self.K2_GetActorLocation`)))
        (:`then_1`
          (`self.SetActorHiddenInGame` true)
          (`KismetSystemLibrary.Delay` 2.0)
          (`self.SetActorHiddenInGame` false))))))

(fn `UserConstructionScript`)