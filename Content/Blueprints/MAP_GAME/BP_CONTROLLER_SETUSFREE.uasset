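; Player controller for the SETUSFREE game mode, handling respawning, the in-game HUD and chat.
; A looping server timer respawns and possesses a player character at the first PlayerStart, or a temporary scaled-up giant at a fixed spot while HasVictory is set.
; Insert or Escape shows the HUD widget, whose close event collapses it.
; ADD_CHAT forwards messages to the game mode, and a CHATS RepNotify refreshes the widget's chat.
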(event `CHECK_DEAD`
  (`/Engine/EditorBlueprintResources/StandardMacros.IsValid` (`self.K2_GetPawn`)
    (:`Is Not Valid`
      (bind _outactors (`GameplayStatics.GetAllActorsOfClass` "/Script/Engine.PlayerStart"))
      (if (`self.bHasVictory`)
        (bind _returnvalue (`|SpawnActorFromClass` "/Game/Blueprints/MAP_GAME/CHAR_GIANT.CHAR_GIANT_C" (`KismetMathLibrary.MakeTransform` (-14479.0 10167.0 500.0) (struct) (5.0 5.0 5.0)) true))
        (`self.Possess` self _returnvalue)
        (`self.SetLifeSpan` _returnvalue 30.0)
        (`KismetSystemLibrary.Delay` 20.0)
        (set `self.bHasVictory` false)
        (else
          (bind _returnvalue_2 (`|SpawnActorFromClass` "/Game/Blueprints/MAP_GAME/CHAR_PLAYER.CHAR_PLAYER_C" (`KismetMathLibrary.MakeTransform` (`self.K2_GetActorLocation` (`KismetArrayLibrary.Array_Get` _outactors)))))
          (`self.Possess` self _returnvalue_2))))))

(event `self.ReceiveBeginPlay`
  (`|ExecutionSequence`
    (:`then_0`
      (`/Engine/EditorBlueprintResources/ActorMacros.Switch Has Authority`
        (:`Authority`
          (`KismetSystemLibrary.K2_SetTimer` null "CHECK_DEAD" 1.0 true))))
    (:`then_1`
      (`/Engine/EditorBlueprintResources/StandardMacros.IsValid` (`self.GetHUD`)
        (:`Is Valid`
          (bind _returnvalue (`|CreateWidget` "/Game/Blueprints/MAP_GAME/GAME_UMG_HUD.GAME_UMG_HUD_C" self))
          (bind _output_get (set `self.hudGAME` _returnvalue))
          (`UserWidget.AddToViewport` _output_get 0)
          (`Widget.SetVisibility` _output_get "Collapsed")
          (add `/Game/Blueprints/MAP_GAME/GAME_UMG_HUD.ClosePLZ` _returnvalue (delegate `CLOSE_ESC`)))))))

(event `CLOSE_ESC`
  (`Widget.SetVisibility` (`self.hudGAME`) "Collapsed"))

(event `self.ReceiveEndPlay`
  (params (EndPlayReason :type "EngineTypes.EEndPlayReason Enum" :default "ActorDestroyed"))
  (`Widget.RemoveFromParent` (`self.hudGAME`)))

(event `self.ReceiveTick`
  (params (DeltaSeconds :type "Float (single-precision)")))

(event `Key|Insert`
  (:`Pressed`
    (`Widget.SetVisibility` (`self.hudGAME`) "Visible" :!label _label)))

(event `Key|Escape`
  (:`Pressed`
    (goto _label)))

(event `ADD_CHAT`
  (params (theCHAT :type "/Game/Blueprints/MAP_GAME/CONFIG/CHAT_STRUCT Structure"))
  (bind _asbp_gamemode_setusfree (cast `/Game/Blueprints/MAP_GAME/BP_GAMEMODE_SETUSFREE` (`GameplayStatics.GetGameMode`)))
  (`/Game/Blueprints/MAP_GAME/BP_GAMEMODE_SETUSFREE.ADD_CHAT` _asbp_gamemode_setusfree theCHAT))

(fn `OnRep_CHATS`
  (bind _hudgame (`self.hudGAME`))
  (`/Engine/EditorBlueprintResources/StandardMacros.IsValid` _hudgame
    (:`Is Valid`
      (`/Game/Blueprints/MAP_GAME/GAME_UMG_HUD.Refresh Chat` _hudgame (`self.CHATS`)))))

(fn `UserConstructionScript`)