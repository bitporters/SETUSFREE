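; A networked enemy fireball projectile that flies along its facing and explodes on overlapping anything but its Owner.
; An attack from a non-owner makes the attacker the Owner and reverses velocity, with a half-second lockout between reflections; the Owner's attack detonates it.
; Detonation disables effect and collision, the authority sets a replicated transform whose OnRep spawns BP_Explosion, and the actor is destroyed after a short delay.
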(event `Hit with attack_1`
  (params (`Impact Vector` :type "Object.Vector Structure") (`Weapon damage` :type "Float (double-precision)") (`Weapon weight` :type "Float (double-precision)") (Attacker :type "Actor Object Reference"))
  (bind _projectile_component (`self.Projectile component`))
  (bind _fireball (`self.Fireball`))
  (if (!= Attacker (`self.Owner`))
    (set `self.Owner` Attacker)
    (`/Engine/EditorBlueprintResources/StandardMacros.DoOnce` false :!label _label
      (:`Completed`
        (`|ExecutionSequence`
          (:`then_0`
            (set `MovementComponent.Velocity` (* (`MovementComponent.Velocity` _projectile_component) -1.0) _projectile_component))
          (:`then_1`
            (`KismetSystemLibrary.Delay` 0.5)
            (goto _label :!via `Reset`)))))
    (else
      (`ActorComponent.SetActive` (`self.Effect`) false false :!label _label_2)
      (`PrimitiveComponent.SetCollisionEnabled` _fireball "NoCollision")
      (`PrimitiveComponent.SetCollisionEnabled` (`self.Weapon collision`) "NoCollision")
      (`/Engine/EditorBlueprintResources/ActorMacros.Switch Has Authority`
        (:`Authority`
          (set `self.Rep_ExplosionTransform` (`KismetMathLibrary.MakeTransform` (+ (`self.K2_GetActorLocation`) (* (`KismetMathLibrary.Conv_RotatorToVector` (`self.K2_GetActorRotation`)) -20.0)))))
        (:`Remote`
          _))
      (`ActorComponent.K2_DestroyComponent` _fireball)
      (`KismetSystemLibrary.Delay` 1.0)
      (`self.K2_DestroyActor`))))

(event `self.ReceiveBeginPlay`
  (set `MovementComponent.Velocity` (`KismetMathLibrary.GreaterGreater_VectorRotator` (`self.Initial Velocity`) (`self.K2_GetActorRotation`)) (`self.Projectile component`))
  (`GameplayStatics.PlaySoundAttached` "/Game/RESOURCES/ExampleContent/Audio/Room_03/Arcade_Enemy_Destroyed_Cue.Arcade_Enemy_Destroyed_Cue" (`self.Fireball`) "None" (0.0 0.0 0.0) "EAttachLocation::KeepRelativeOffset" false 1.0 1.0))

(event `self.Fireball.OnComponentBeginOverlap`
  (params (OtherActor :type "Actor Object Reference") (OtherComp :type "PrimitiveComponent Object Reference") (OtherBodyIndex :type Integer) (bFromSweep :type Boolean) (SweepResult :type "EngineTypes.HitResult Structure (by ref)"))
  (if (not (== (`self.Owner`) OtherActor))
    (goto _label_2)))

(fn `Hit with attack`
  (params (`Impact vector` :type "Object.Vector Structure") (`Weapon damage` :type "Float (double-precision)") (`Weapon weight` :type "Float (double-precision)") (Attacker :type "Actor Object Reference"))
  (returns (bWasDamaged :type Boolean))
  (return false))

(fn `OnRep_Rep_ExplosionTransform`
  (`|SpawnActorFromClass` "/Game/Blueprints/MAP_GAME/Game/BP_Explosion.BP_Explosion_C" (`self.Rep_ExplosionTransform`) true (`self.SMall explosion`) (`self.Owner`)))

(fn `UserConstructionScript`)