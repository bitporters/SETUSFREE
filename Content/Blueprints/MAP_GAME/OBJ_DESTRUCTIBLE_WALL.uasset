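; A destructible wall obstacle that the player can blow up while holding a wall-breaker ability.
; When CHAR_PLAYER overlaps the trigger sphere with CanExplodeWall set, it consumes that flag, deactivates the player's wallbreaker effect and calls ExplodeWall.
; ExplodeWall fractures both destructible meshes with radius damage, disables their collision, and spawns an oversized explosion particle and sound at the explosion point.
; After a short delay, both destructible components are destroyed.
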(event `self.ReceiveBeginPlay`)

(event `self.ReceiveActorBeginOverlap`
  (params (OtherActor :type "Actor Object Reference")))

(event `self.ReceiveTick`
  (params (DeltaSeconds :type "Float (single-precision)")))

(event `self.Sphere.OnComponentBeginOverlap`
  (params (OtherActor :type "Actor Object Reference") (OtherComp :type "PrimitiveComponent Object Reference") (OtherBodyIndex :type Integer) (bFromSweep :type Boolean) (SweepResult :type "EngineTypes.HitResult Structure (by ref)"))
  (bind _aschar_player (cast `/Game/Blueprints/MAP_GAME/CHAR_PLAYER` OtherActor))
  (if (`/Game/Blueprints/MAP_GAME/CHAR_PLAYER.bCanExplodeWall` _aschar_player)
    (set `/Game/Blueprints/MAP_GAME/CHAR_PLAYER.bCanExplodeWall` false _aschar_player)
    (`ActorComponent.Deactivate` (`/Game/Blueprints/MAP_GAME/CHAR_PLAYER.p_wallbreaker` _aschar_player))
    (`self.ExplodeWall`)
    (`KismetSystemLibrary.Delay` 2.0)
    (`ActorComponent.K2_DestroyComponent` (`self.Destructible`))
    (`ActorComponent.K2_DestroyComponent` (`self.Destructible1`))))

(fn `ExplodeWall`
  (bind _destructible (`self.Destructible`))
  (bind _destructible1 (`self.Destructible1`))
  (bind _returnvalue (`SceneComponent.K2_GetComponentLocation` (`self.objExplosionPoint`)))
  (`DestructibleComponent.ApplyRadiusDamage` _destructible1 1000.0 _returnvalue 1000.0 1000.0 true)
  (`DestructibleComponent.ApplyRadiusDamage` _destructible 1000.0 _returnvalue 1000.0 1000.0 true)
  (`PrimitiveComponent.SetCollisionEnabled` _destructible1 "NoCollision")
  (`PrimitiveComponent.SetCollisionEnabled` _destructible "NoCollision")
  (bind _returnvalue_2 (`GameplayStatics.SpawnEmitterAtLocation` "/Game/RESOURCES/Effects/Particle_Systems/P_Explosion_Bomb.P_Explosion_Bomb" _returnvalue))
  (`SceneComponent.SetWorldScale3D` _returnvalue_2 (100.0 100.0 100.0))
  (`GameplayStatics.PlaySoundAtLocation` "/Game/RESOURCES/ExampleContent/Audio/Room_03/Arcade_Explosion_Sweet_02.Arcade_Explosion_Sweet_02" _returnvalue))

(fn `UserConstructionScript`)