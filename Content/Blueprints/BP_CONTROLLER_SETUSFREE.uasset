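; BP_CONTROLLER_SETUSFREE is a controller that automatically respawns its player character.
; On BeginPlay, the authority side starts a looping one-second timer that polls CHECK_DEAD.
; When no valid controlled pawn exists, CHECK_DEAD spawns a CHAR_PLAYER at the location of the first PlayerStart found, with zero rotation, and possesses it.
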(event `self.ReceiveBeginPlay`
  (`/Engine/EditorBlueprintResources/ActorMacros.Switch Has Authority`
    (:`Authority`
      (`KismetSystemLibrary.K2_SetTimer` null "CHECK_DEAD" 1.0 true))))

(event `CHECK_DEAD`
  (`/Engine/EditorBlueprintResources/StandardMacros.IsValid` (`self.K2_GetPawn`)
    (:`Is Not Valid`
      (bind _outactors (`GameplayStatics.GetAllActorsOfClass` "/Script/Engine.PlayerStart"))
      (bind _returnvalue (`|SpawnActorFromClass` "/Game/Blueprints/CHAR_PLAYER.CHAR_PLAYER_C" (`KismetMathLibrary.MakeTransform` (`self.K2_GetActorLocation` (`KismetArrayLibrary.Array_Get` _outactors)))))
      (`self.Possess` self _returnvalue))))

(event `self.ReceiveTick`
  (params (DeltaSeconds :type "Float (single-precision)")))

(fn `UserConstructionScript`)