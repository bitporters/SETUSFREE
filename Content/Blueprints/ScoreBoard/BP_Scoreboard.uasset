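; Two-player VR scoreboard actor that shows calibration status, live scores and the winner, and drives its camera from the headset pose each tick.
; RepNotify variables feed events that switch Waiting to Ready materials and set each score through a material "number" parameter.
; Once both players calibrate, chained timelines fade the instructions, raise the player anchor and reveal scores.
; PlayerWins fades scores and displays the victor; ResetScoreboard restores the waiting layout.
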(event `self.ReceiveBeginPlay`
  (set `self.OriginalCamOffset` (`SceneComponent.RelativeLocation` (`self.Camera1`))))

(event `self.ReceiveTick`
  (params (DeltaSeconds :type "Float (single-precision)"))
  (bind (_devicerotation _deviceposition) (`HeadMountedDisplayFunctionLibrary.GetOrientationAndPosition`))
  (bind _camera1 (`self.Camera1`))
  (`SceneComponent.K2_SetRelativeLocation` _camera1 (+ _deviceposition (`self.OriginalCamOffset`)) false)
  (`SceneComponent.K2_SetRelativeRotation` _camera1 _devicerotation false))

(event `Player Wins`
  (bind _victory_player (`self.Victory player`))
  (bind (_direction _newtrack_0) (`Timeline|Timeline_3` :!via `PlayFromStart`)
    (:`Update`
      (`MaterialInstanceDynamic.SetScalarParameterValue` (`self.P1 Score Mat`) "opacity" (`KismetMathLibrary.Lerp` 1.0 0.0 _newtrack_0))
      (`MaterialInstanceDynamic.SetScalarParameterValue` (`self.P2 Score Mat`) "opacity" (`KismetMathLibrary.Lerp` 1.0 0.0 _newtrack_0)))
    (:`Finished`
      (if (> (`self.Player 1 Score`) (`self.Player 2 Score`))
        (set `self.Player to lerp` (`self.P1`))
        (`PrimitiveComponent.SetMaterial` _victory_player 0 "/Game/Blueprints/ScoreBoard/M_Text_PLayer1.M_Text_PLayer1")
        (else
          (set `self.Player to lerp` (`self.P2`))
          (`PrimitiveComponent.SetMaterial` _victory_player 0 "/Game/Blueprints/ScoreBoard/M_Text_PLayer2.M_Text_PLayer2")))
      (`SceneComponent.SetHiddenInGame` (`self.P1`) true false)
      (`SceneComponent.SetHiddenInGame` (`self.P2`) true false)
      (`SceneComponent.SetHiddenInGame` (`self.Victory player`) false false)
      (`SceneComponent.SetHiddenInGame` (`self.Wins`) false false))))

(event `Reset Scoreboard`
  (`MaterialInstanceDynamic.SetScalarParameterValue` (`self.P2 Score Mat`) "number" 0.0)
  (`MaterialInstanceDynamic.SetScalarParameterValue` (`self.P1 Score Mat`) "number" 0.0)
  (`SceneComponent.K2_SetRelativeLocation` (`self.P Anchor`) (0.0 0.0 0.0) false)
  (`SceneComponent.SetHiddenInGame` (`self.P2 Score`) true false)
  (`SceneComponent.SetHiddenInGame` (`self.P1 Score`) true false)
  (`SceneComponent.SetHiddenInGame` (`self.P2Waiting`) false false)
  (`SceneComponent.SetHiddenInGame` (`self.P1Waiting`) false false)
  (`SceneComponent.SetHiddenInGame` (`self.Directions`) false false)
  (`SceneComponent.SetHiddenInGame` (`self.P1`) false false)
  (`SceneComponent.SetHiddenInGame` (`self.P2`) false false)
  (`MaterialInstanceDynamic.SetScalarParameterValue` (`self.Directions Mat`) "Opacity" 1.0)
  (`MaterialInstanceDynamic.SetScalarParameterValue` (`self.P2Waiting mat`) "Opacity" 1.0)
  (`MaterialInstanceDynamic.SetScalarParameterValue` (`self.P1 Waiting Mat`) "Opacity" 1.0)
  (`SceneComponent.SetHiddenInGame` (`self.P2Dots`) false false)
  (`SceneComponent.SetHiddenInGame` (`self.P1Dots`) false false)
  (`SceneComponent.SetHiddenInGame` (`self.Victory player`) true false)
  (`SceneComponent.SetHiddenInGame` (`self.Wins`) true false)
  (`MaterialInstanceDynamic.SetScalarParameterValue` (`self.P1 Score Mat`) "opacity" 1.0)
  (`MaterialInstanceDynamic.SetScalarParameterValue` (`self.P2 Score Mat`) "opacity" 1.0)
  (`KismetSystemLibrary.Delay` 0.0)
  (`PrimitiveComponent.SetMaterial` (`self.P1Waiting`) 0 "/Game/Blueprints/ScoreBoard/M_Text_Wait.M_Text_Wait")
  (`PrimitiveComponent.SetMaterial` (`self.P2Waiting`) 0 "/Game/Blueprints/ScoreBoard/M_Text_Wait.M_Text_Wait")
  (`SceneComponent.SetHiddenInGame` (`self.P1Dots`) false false)
  (`SceneComponent.SetHiddenInGame` (`self.P1Dots`) false false))

(event `Player1ScoreUpdated`
  (params (Score :type Integer))
  (`MaterialInstanceDynamic.SetScalarParameterValue` (`self.P1 Score Mat`) "number" (`KismetMathLibrary.Conv_IntToDouble` Score)))

(event `Player2ScoreUpdated`
  (params (Score :type Integer))
  (`MaterialInstanceDynamic.SetScalarParameterValue` (`self.P2 Score Mat`) "number" (`KismetMathLibrary.Conv_IntToDouble` Score)))

(event `Player1Calibrated`
  (params (Calibrated :type Boolean))
  (`PrimitiveComponent.SetMaterial` (`self.P1Waiting`) 0 "/Game/Blueprints/ScoreBoard/M_Text_Ready.M_Text_Ready")
  (`SceneComponent.SetHiddenInGame` (`self.P1Dots`) true false)
  (if (and (`self.Player 1 Calibrated`) (`self.Player 2 Calibrated`)) :!label _label
    (bind (_direction _newtrack_0) (`Timeline|Timeline_0` :!via `PlayFromStart`)
      (:`Update`
        (`MaterialInstanceDynamic.SetScalarParameterValue` (`self.Directions Mat`) "Opacity" (`KismetMathLibrary.Lerp` 1.0 0.0 _newtrack_0))
        (`MaterialInstanceDynamic.SetScalarParameterValue` (`self.P2Waiting mat`) "Opacity" (`KismetMathLibrary.Lerp` 1.0 0.0 _newtrack_0))
        (`MaterialInstanceDynamic.SetScalarParameterValue` (`self.P1 Waiting Mat`) "Opacity" (`KismetMathLibrary.Lerp` 1.0 0.0 _newtrack_0)))
      (:`Finished`
        (`SceneComponent.SetHiddenInGame` (`self.P2Waiting`) true false)
        (`SceneComponent.SetHiddenInGame` (`self.P1Waiting`) true false)
        (`SceneComponent.SetHiddenInGame` (`self.Directions`) true false)
        (bind (_direction_2 _newtrack_1) (`Timeline|Timeline_1` :!via `PlayFromStart`)
          (:`Update`
            (`SceneComponent.K2_SetRelativeLocation` (`self.P Anchor`) (`KismetMathLibrary.VLerp` (0.0 0.0 0.0) (0.0 0.0 30.0) _newtrack_1) false))
          (:`Finished`
            (`SceneComponent.SetHiddenInGame` (`self.P2 Score`) false false)
            (`SceneComponent.SetHiddenInGame` (`self.P1 Score`) false false)))))))

(event `Player2Calibrated`
  (params (Calibrated :type Boolean))
  (`PrimitiveComponent.SetMaterial` (`self.P2Waiting`) 0 "/Game/Blueprints/ScoreBoard/M_Text_Ready.M_Text_Ready")
  (`SceneComponent.SetHiddenInGame` (`self.P2Dots`) true false)
  (goto _label))

(event `Player1Ready`
  (params (Ready :type Boolean)))

(event `Player2Ready`
  (params (Ready :type Boolean)))

(fn `OnRep_Player 1 Calibrated`
  (`self.Player1Calibrated` (`self.Player 1 Calibrated`)))

(fn `OnRep_Player 1 Ready`
  (`self.Player1Ready` (`self.Player 1 Ready`)))

(fn `OnRep_Player 1 Score`
  (`self.Player1ScoreUpdated` (`self.Player 1 Score`)))

(fn `OnRep_Player 2 Calibrated`
  (`self.Player2Calibrated` (`self.Player 2 Calibrated`)))

(fn `OnRep_Player 2 Ready`
  (`self.Player2Ready` (`self.Player 2 Ready`)))

(fn `OnRep_Player 2 Score`
  (`self.Player2ScoreUpdated` (`self.Player 2 Score`)))

(fn `UserConstructionScript`
  (bind _returnvalue (`PrimitiveComponent.CreateDynamicMaterialInstance` (`self.P1Waiting`) 0 null))
  (set `self.P1 Waiting Mat` _returnvalue)
  (bind _returnvalue_2 (`PrimitiveComponent.CreateDynamicMaterialInstance` (`self.P2Waiting`) 0 null))
  (set `self.P2Waiting mat` _returnvalue_2)
  (bind _returnvalue_3 (`PrimitiveComponent.CreateDynamicMaterialInstance` (`self.Directions`) 0 null))
  (set `self.Directions Mat` _returnvalue_3)
  (bind _returnvalue_4 (`PrimitiveComponent.CreateDynamicMaterialInstance` (`self.P1 Score`) 0 null))
  (set `self.P1 Score Mat` _returnvalue_4)
  (bind _returnvalue_5 (`PrimitiveComponent.CreateDynamicMaterialInstance` (`self.P2 Score`) 0 null))
  (set `self.P2 Score Mat` _returnvalue_5)
  (set `self.P1 Transform` (`SceneComponent.K2_GetComponentToWorld` (`self.P1`)))
  (set `self.P2 Transform` (`SceneComponent.K2_GetComponentToWorld` (`self.P2`))))