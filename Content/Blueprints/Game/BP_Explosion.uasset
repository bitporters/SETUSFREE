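; BP_Explosion is a short-lived explosion actor whose type selects the particle effect, damage, radius and force.
; On BeginPlay it enables and nudges its trigger to catch overlaps, fires a radial impulse, then self-destroys after a brief delay.
; Overlapping BPI_Weapon_Interactions actors other than the source qualify for curve-based distance falloff of damage and force.
; A DoOnce limits this to one hit message per explosion; scorch decal code is disconnected.
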(event `self.ReceiveBeginPlay`
  (bind _returnvalue (`self.K2_GetActorLocation`))
  (bind _explosion_trigger (`self.Explosion trigger`))
  (switch `/Game/Blueprints/Game/Enum_Explosion_Type` (`self.explosion type`)
    (:`Small_Explosion`
      (`GameplayStatics.SpawnEmitterAtLocation` "/Game/RESOURCES/Effects/Particle_Systems/P_Explosion_Bomb.P_Explosion_Bomb" _returnvalue)
      (set `self.Explosion damage` 25.0)
      (set `self.Explosion radius` 40.0)
      (set `self.Explosion force` 50.0))
    (:`Medium_Explosion`
      ;[1 1 1] Not used atm
      (`GameplayStatics.SpawnEmitterAtLocation` "/Game/RESOURCES/Effects/Particle_Systems/P_Explosion_Small.P_Explosion_Small" _returnvalue)
      (set `self.Explosion damage` 40.0)
      (set `self.Explosion radius` 160.0)
      (set `self.Explosion force` 60.0))
    (:`Fireball_Explosion`
      (`GameplayStatics.SpawnEmitterAtLocation` "/Game/RESOURCES/Effects/Particle_Systems/P_Explosion_Fireball.P_Explosion_Fireball" _returnvalue)
      (set `self.Explosion damage` 30.0)
      (set `self.Explosion radius` 140.0)
      (set `self.Explosion force` 40.0)))
  (`PrimitiveComponent.SetCollisionEnabled` _explosion_trigger "QueryOnly")
  (`SceneComponent.K2_AddLocalOffset` _explosion_trigger (0.0 0.0 0.1) false)
  (`RadialForceComponent.FireImpulse` (`self.RadialForce1`))
  (`KismetSystemLibrary.Delay` 0.2)
  (`self.K2_DestroyActor`))

(event `self.Explosion trigger.OnComponentBeginOverlap`
  (params (OtherActor :type "Actor Object Reference") (OtherComp :type "PrimitiveComponent Object Reference") (OtherBodyIndex :type Integer) (bFromSweep :type Boolean) (SweepResult :type "EngineTypes.HitResult Structure (by ref)"))
  (bind _returnvalue (`CurveFloat.GetFloatValue` (`self.Radius curve`) (`KismetMathLibrary.MapRange` (`self.GetDistanceTo` OtherActor) 0.0 (`self.Explosion radius`) 1.0 0.0)))
  (if (and (!= OtherActor (`self.Source actor`)) (`KismetSystemLibrary.DoesImplementInterface` OtherActor "/Game/Blueprints/Game/BPI_Weapon_Interactions.BPI_Weapon_Interactions_C"))
    (set `self.Hit actor` OtherActor)
    (if (> _returnvalue 0.1)
      (`/Engine/EditorBlueprintResources/StandardMacros.DoOnce` false
        (:`Completed`
          (message `/Game/Blueprints/Game/BPI_Weapon_Interactions.Hit with attack` (`self.Hit actor`) (`KismetMathLibrary.Normal` (- (`self.K2_GetActorLocation` OtherActor) (`self.K2_GetActorLocation`))) (* _returnvalue (`self.Explosion damage`)) (* _returnvalue (`self.Explosion force`)) self))))))

(fn `Hit with attack`
  (params (`Impact vector` :type "Object.Vector Structure") (`Weapon damage` :type "Float (double-precision)") (`Weapon weight` :type "Float (double-precision)") (Attacker :type "Actor Object Reference"))
  (returns (bWasDamaged :type Boolean))
  (return false))

(fn `UserConstructionScript`)